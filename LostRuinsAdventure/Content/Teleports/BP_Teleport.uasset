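; Level-exit teleport actor that moves the player from Level_1 to Level_2 and ends the game at Level_2.
; When an actor tagged Player overlaps its box, it copies the character's collected artifact list into the LRA_GI game instance to persist across levels.
; In Level_1 it opens Level_2; in Level_2 it shows the WB_Complete widget with the artifact count and destroys the player character.
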(event OnComponentBeginOverlap(Box)
  (params (OverlappedComponent :type Primitive%20Component%20Object%20Reference) (OtherActor :type Actor%20Object%20Reference) (OtherComp :type Primitive%20Component%20Object%20Reference) (OtherBodyIndex :type Integer) (bFromSweep :type Boolean) (SweepResult :type Hit%20Result%20Structure%20%28by%20ref%29))
  ;[1 1 1] Teleport To Next Level
  (if (Actor|ActorHasTag OtherActor "Player")
    (bind _aslra_gi (Utilities|Casting|CastToLRA_GI (Game|GetGameInstance)))
    (bind _ascharacter_bp (Utilities|Casting|CastToCharacter_BP (Game|GetPlayerCharacter 0)))
    (Variables|/Script/LostRuinsAdventure.LRAGameInstance|SetArtifactList _aslra_gi (Variables|/Script/LostRuinsAdventure.CollectArtifact|GetArtifactList (Variables|/Game/Characters/Player/Character_BP.Character_BP_C|GetCollectArtifact _ascharacter_bp)))
    (bind _returnvalue (Game|GetCurrentLevelName true))
    (if (Utilities|Enum|Equal(Enum) _returnvalue "Level_2")
      (bind _returnvalue_2 (UserInterface|CreateWidget "/Game/UI/Player/WB_Complete.WB_Complete_C"))
      (bind _output_get (Variables|Default|SetCompleteHUD _returnvalue_2))
      (UserInterface|Viewport|AddtoViewport _output_get 0)
      (bind _ascharacter_bp_2 (Utilities|Casting|CastToCharacter_BP (Game|GetPlayerCharacter 0)))
      (Variables|/Game/UI/Player/WB_Complete.WB_Complete_C|SetTotalArtifact (Variables|Default|GetCompleteHUD) (Utilities|Array|Length (Variables|/Script/LostRuinsAdventure.CollectArtifact|GetArtifactList (Variables|/Game/Characters/Player/Character_BP.Character_BP_C|GetCollectArtifact _ascharacter_bp_2))))
      (Actor|DestroyActor _ascharacter_bp_2)
      (elif (Utilities|Enum|Equal(Enum) _returnvalue "Level_1")
        (Game|OpenLevel(byName) "Level_2")))))

(event EventBeginPlay)

(event Collision|EventActorBeginOverlap
  (params (OtherActor :type Actor%20Object%20Reference)))

(event EventTick
  (params (DeltaSeconds :type Float%20%28single-precision%29)))

(fn ConstructionScript)