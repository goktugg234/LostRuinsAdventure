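; Player character Blueprint that drives the HUD for health and artifact count and handles damage feedback.
; On BeginPlay it creates the HUD and restores the collected artifact list from the LRA_GI game instance.
; Health and artifact events refresh the HUD.
; Damage triggers camera shake and a hit effect widget, subtracts from the displayed health, and shows the death screen with a cursor at zero.
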(event EventBeginPlay
  ;[1 1 1] HUD Display
  (bind _returnvalue (UserInterface|CreateWidget "/Game/UI/Player/WB_HUD.WB_HUD_C"))
  (bind _output_get (Variables|Default|SetHUD _returnvalue))
  (UserInterface|Viewport|AddtoViewport _output_get 0)
  (Variables|/Game/UI/Player/WB_HUD.WB_HUD_C|SetHealth _output_get (Variables|/Script/LostRuinsAdventure.LRAHealthComponent|GetHealth (Variables|Default|GetLRAHealth)))
  ;[1 1 1] Set Artifact Number To Instance
  (bind _aslra_gi (Utilities|Casting|CastToLRA_GI (Game|GetGameInstance)))
  (bind _output_get_2 (Variables|/Script/LostRuinsAdventure.CollectArtifact|SetArtifactList (Variables|Default|GetCollectArtifact) (Variables|/Script/LostRuinsAdventure.LRAGameInstance|GetArtifactList _aslra_gi)))
  (Variables|/Game/UI/Player/WB_HUD.WB_HUD_C|SetArtifact (Variables|Default|GetHUD) (Utilities|Array|Length _output_get_2)))

(event EventOnHealthUpdated
  ;[1 1 1] Update Health
  (Variables|/Game/UI/Player/WB_HUD.WB_HUD_C|SetHealth (Variables|Default|GetHUD) (Variables|/Script/LostRuinsAdventure.LRAHealthComponent|GetHealth (Variables|Default|GetLRAHealth))))

(event Game|Damage|EventAnyDamage
  (params (Damage :type Float%20%28single-precision%29) (DamageType :type Damage%20Type%20Object%20Reference) (InstigatedBy :type Controller%20Object%20Reference) (DamageCauser :type Actor%20Object%20Reference))
  ;[1 1 1] Get Damage
  (bind _output_get (Variables|/Game/UI/Player/WB_HUD.WB_HUD_C|SetHealth (Variables|Default|GetHUD) (- (Variables|/Script/LostRuinsAdventure.LRAHealthComponent|GetHealth (Variables|Default|GetLRAHealth)) Damage)))
  (Camera|PlayWorldCameraShake "/Script/Engine.CameraShakeBase" "0, 0, 0" 0.0 6e+02)
  (bind _returnvalue (UserInterface|CreateWidget "/Game/UI/Player/WB_HitEffect.WB_HitEffect_C"))
  (UserInterface|Viewport|AddtoViewport _returnvalue 0)
  (if (<= _output_get 0.0)
    (bind _returnvalue_2 (UserInterface|CreateWidget "/Game/UI/Player/WB_DeathScreen.WB_DeathScreen_C"))
    (UserInterface|Viewport|AddtoViewport _returnvalue_2 0)
    (Variables|/Script/Engine.PlayerController|SetbShowMouseCursor (Game|GetPlayerController 0) true)))

(event EventOnArtifactAdded
  (params (Artifact :type Integer))
  ;[1 1 1] Artifact Added
  (Variables|/Game/UI/Player/WB_HUD.WB_HUD_C|SetArtifact (Variables|Default|GetHUD) Artifact))

(fn ConstructionScript)