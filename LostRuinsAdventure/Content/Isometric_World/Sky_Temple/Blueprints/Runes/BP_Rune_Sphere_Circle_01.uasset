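; Decorative Sky Temple rune sphere/circle actor that continuously spins five static mesh parts.
; On BeginPlay it starts five timelines, one per mesh, each adding a vector-driven local rotation to its mesh on every update.
; Each timeline restarts itself from the start when finished, so the motion loops indefinitely.
; The rotation is applied per update without delta-time scaling, so spin speed depends on frame rate.
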(event EventBeginPlay
  (Utilities|FlowControl|Sequence
    (:then_0
      (bind _rotation (Timeline|Rotation Play)
        (:Update
          (Transformation|AddLocalRotation (Variables|Default|GetStaticMesh1) (Math|Rotator|MakeRotator (.X (Math|Vector|BreakVector _rotation)) (.Y (Math|Vector|BreakVector _rotation)) (.Z (Math|Vector|BreakVector _rotation))) false false))
        (:Finished
          (Utilities|FlowControl|Sequence
            (:then_0
              (Timeline|Rotation PlayFromStart))))))
    (:then_1
      (bind _rotation_2 (Timeline|Timeline_0 Play)
        (:Update
          (Transformation|AddLocalRotation (Variables|Default|GetStaticMesh2) (Math|Rotator|MakeRotator (.X (Math|Vector|BreakVector _rotation_2)) (.Y (Math|Vector|BreakVector _rotation_2)) (.Z (Math|Vector|BreakVector _rotation_2))) false false))
        (:Finished
          (Utilities|FlowControl|Sequence
            (:then_0
              (Timeline|Timeline_0 PlayFromStart))))))
    (:then_2
      (bind _rotation_3 (Timeline|Timeline_1 Play)
        (:Update
          (Transformation|AddLocalRotation (Variables|Default|GetStaticMesh3) (Math|Rotator|MakeRotator (.X (Math|Vector|BreakVector _rotation_3)) (.Y (Math|Vector|BreakVector _rotation_3)) (.Z (Math|Vector|BreakVector _rotation_3))) false false))
        (:Finished
          (Utilities|FlowControl|Sequence
            (:then_0
              (Timeline|Timeline_1 PlayFromStart))))))
    (:then_3
      (bind _rotation_4 (Timeline|Timeline_2 Play)
        (:Update
          (Transformation|AddLocalRotation (Variables|Default|GetStaticMesh4) (Math|Rotator|MakeRotator (.X (Math|Vector|BreakVector _rotation_4)) (.Y (Math|Vector|BreakVector _rotation_4)) (.Z (Math|Vector|BreakVector _rotation_4))) false false))
        (:Finished
          (Utilities|FlowControl|Sequence
            (:then_0
              (Timeline|Timeline_2 PlayFromStart))))))
    (:then_4
      (bind _rotation_5 (Timeline|Timeline_3 Play)
        (:Update
          (Transformation|AddLocalRotation (Variables|Default|GetStaticMesh5) (Math|Rotator|MakeRotator (.X (Math|Vector|BreakVector _rotation_5)) (.Y (Math|Vector|BreakVector _rotation_5)) (.Z (Math|Vector|BreakVector _rotation_5))) false false))
        (:Finished
          (Utilities|FlowControl|Sequence
            (:then_0
              (Timeline|Timeline_3 PlayFromStart))))))))

(fn ConstructionScript)